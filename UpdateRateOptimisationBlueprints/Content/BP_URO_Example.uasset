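; Example Blueprint showing ways to apply animation Update Rate Optimisation (URO) to a skeletal mesh.
; BeginPlay applies a Data Asset preset using visible distance factor thresholds.
; Unwired alternatives show setup by struct or by two custom events that set LOD frame-skip or distance-threshold mode node by node, with interpolation and non-rendered update rate.
; Other disconnected nodes form a catalogue of URO setters and getters, plus debug prints for current settings.
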(event `self.ReceiveBeginPlay`
  ;[0.1 0.1 0.1] Example Setup - Begin Play - Choose a method to apply URO
  (`parent.ReceiveBeginPlay`)
  ;;[0.6968 0.3538 1] 1 - Assign URO via Data Asset
  (`UpdateRateOptimisationBlueprintsBPLibrary.SetUpdateRateOptimisationByDataAsset` (`self.SkeletalMesh`) true "/UpdateRateOptimisationBlueprints/DA_URO_VisibleDistanceFactorThresholds.DA_URO_VisibleDistanceFactorThresholds"))

(event `self.ReceiveTick`
  (params (DeltaSeconds :type "Float (single-precision)"))
  ;[0.1 0 0.04346] Debug Methods
)

(event `LODToFrameSkipMap`
  (bind _skeletalmesh (`self.SkeletalMesh`))
  ;[0.1 0.1 0.1] Individual Node Setup Examples
  ;;[0 0.01474 0.1] EXAMPLE - LOD Optimisation Pipeline by setting each parameter individually
  (`UpdateRateOptimisationBlueprintsBPLibrary.SetEnableUpdateRateOptimisationsOnSkinnedMesh` _skeletalmesh true)
  (`UpdateRateOptimisationBlueprintsBPLibrary.SetUpdateRateOptimisationMode` _skeletalmesh "LODToFrameSkipMap")
  (`UpdateRateOptimisationBlueprintsBPLibrary.SetLODToFrameSkipArray` _skeletalmesh (`|MakeArray` 0 3 6 12 15))
  (`UpdateRateOptimisationBlueprintsBPLibrary.SetInterpolateSkippedFrames` _skeletalmesh true)
  (`UpdateRateOptimisationBlueprintsBPLibrary.SetMaxEvalRateForInterpolation` _skeletalmesh 15)
  (`UpdateRateOptimisationBlueprintsBPLibrary.SetBaseNonRenderedUpdateRate` null 20))

(event `VisibleDistanceFactorThreshold`
  (bind _skeletalmesh (`self.SkeletalMesh`))
  ;[0.1 0.1 0.1] Individual Node Setup Examples
  ;;[0.04301 0.1 0.01808] EXAMPLE - Visible Distance Factor Threshold by setting each parameter individually
  (`UpdateRateOptimisationBlueprintsBPLibrary.SetEnableUpdateRateOptimisationsOnSkinnedMesh` _skeletalmesh true)
  (`UpdateRateOptimisationBlueprintsBPLibrary.SetUpdateRateOptimisationMode` _skeletalmesh "VisibleDistanceFactorThresholds")
  (`UpdateRateOptimisationBlueprintsBPLibrary.SetVisibleDistanceFactorThresholds` _skeletalmesh (`|MakeArray` 0.4 0.3 0.2 0.1 0.05 0.04 0.03 0.02 0.01 0.005 0.00125 0.000625 0.000313 0.000156 7.8e-05 3.9e-05 :!type "Float (single-precision)"))
  (`UpdateRateOptimisationBlueprintsBPLibrary.SetInterpolateSkippedFrames` _skeletalmesh true)
  (`UpdateRateOptimisationBlueprintsBPLibrary.SetMaxEvalRateForInterpolation` _skeletalmesh 15)
  (`UpdateRateOptimisationBlueprintsBPLibrary.SetBaseNonRenderedUpdateRate` null 20))

(fn `UserConstructionScript`)